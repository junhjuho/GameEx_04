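; GM_TargetGame is the game mode for a target game, tracking score and showing a win screen once every target is scored.
; On BeginPlay it sets game-only input, counts BP_Target actors as MaxScore, and creates the WBP_UI score widget.
; AddScore increments CurrentScore and refreshes the UI.
; When CurrentScore equals MaxScore, it shows WBP_EndScreen and switches to UI-only input.
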(event Custom|Add%20Score
  (Utilities|FlowControl|Sequence
    (:then_0
      ;[1 1 1] 점수 증가
      (bind _result (Math|Integer|IncrementInt (Variables|Default|GetCurrentScore))
        (:%20%20
          (Variables|Default|SetCurrentScore _result)
          (Default|UpdateScore (Variables|Default|GetUIRef)))))
    (:then_1
      ;[1 1 1] 게임 승리
      (if (== (Variables|Default|GetCurrentScore) (Variables|Default|GetMaxScore))
        (bind _returnvalue (UserInterface|CreateWidget "/Game/GameEX/UI/WBP_EndScreen.WBP_EndScreen_C"))
        (UserInterface|Viewport|AddtoViewport _returnvalue 0)
        (Input|SetInputModeUIOnly (Game|GetPlayerController 0) _returnvalue "DoNotLock")))))

(event EventBeginPlay
  (Utilities|FlowControl|Sequence
    (:then_0
      ;[1 1 1] Set Input Mode
      (Input|SetInputModeGameOnly (Game|GetPlayerController 0)))
    (:then_1
      (bind _outactors (Actor|GetAllActorsOfClass "/Game/GameEX/Blueprints/BP_Target.BP_Target_C"))
      (Variables|Default|SetMaxScore (Utilities|Array|Length _outactors)))
    (:then_2
      (bind _returnvalue (UserInterface|CreateWidget "/Game/GameEX/UI/WBP_UI.WBP_UI_C"))
      (bind _output_get (Variables|Default|SetUIRef _returnvalue))
      (UserInterface|Viewport|AddtoViewport _output_get 0)
      (Default|UpdateScore _output_get))))

(event EventTick
  (params (DeltaSeconds :type Float%20%28single-precision%29)))

(fn ConstructionScript)